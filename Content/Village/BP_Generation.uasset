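; BP_Generation is a runtime controller that regenerates the procedural village and forest on key press, enabling input from the first player controller on BeginPlay.
; Key 1 randomizes separate PCG graph seed parameters for the village's churches, houses, foliage, trees, market, decoration and offsets, while key 2 randomizes the forest seed.
; Each key finds its BP_Village or BP_Forest actor, then cleans up and force-regenerates that actor's PCG component.
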(event EventBeginPlay
  (Input|EnableInput (Game|GetPlayerController 0)))

(event Collision|EventActorBeginOverlap
  (params (OtherActor :type Actor%20Object%20Reference)))

(event EventTick
  (params (DeltaSeconds :type Float%20%28single-precision%29)))

(event Input|KeyboardEvents|1
  (params (Key :type Key%20Structure :default "None"))
  (:Pressed
    (bind _returnvalue (Actor|GetActorOfClass "/Game/Village/BP_Village.BP_Village_C"))
    (Class|PCGGraphParametersHelpers|SetInt32Parameter (Variables|/Script/PCG.PCGComponent|GetGraphInstance (Variables|/Game/Village/BP_Village.BP_Village_C|GetPCG _returnvalue)) "ChurchSEED" (Math|Random|RandomIntegerinRange -999999999 999999999))
    (Class|PCGGraphParametersHelpers|SetInt32Parameter (Variables|/Script/PCG.PCGComponent|GetGraphInstance (Variables|/Game/Village/BP_Village.BP_Village_C|GetPCG _returnvalue)) "HouseSEED" (Math|Random|RandomIntegerinRange -999999999 999999999))
    (Class|PCGGraphParametersHelpers|SetInt32Parameter (Variables|/Script/PCG.PCGComponent|GetGraphInstance (Variables|/Game/Village/BP_Village.BP_Village_C|GetPCG _returnvalue)) "FoliageSEED" (Math|Random|RandomIntegerinRange -999999999 999999999))
    (Class|PCGGraphParametersHelpers|SetInt32Parameter (Variables|/Script/PCG.PCGComponent|GetGraphInstance (Variables|/Game/Village/BP_Village.BP_Village_C|GetPCG _returnvalue)) "TreeSEED" (Math|Random|RandomIntegerinRange -999999999 999999999))
    (Class|PCGGraphParametersHelpers|SetInt32Parameter (Variables|/Script/PCG.PCGComponent|GetGraphInstance (Variables|/Game/Village/BP_Village.BP_Village_C|GetPCG _returnvalue)) "MarketSEED" (Math|Random|RandomIntegerinRange -999999999 999999999))
    (Class|PCGGraphParametersHelpers|SetInt32Parameter (Variables|/Script/PCG.PCGComponent|GetGraphInstance (Variables|/Game/Village/BP_Village.BP_Village_C|GetPCG _returnvalue)) "DecoSEED" (Math|Random|RandomIntegerinRange -999999999 999999999))
    (Class|PCGGraphParametersHelpers|SetInt32Parameter (Variables|/Script/PCG.PCGComponent|GetGraphInstance (Variables|/Game/Village/BP_Village.BP_Village_C|GetPCG _returnvalue)) "OffsetSEED" (Math|Random|RandomIntegerinRange -999999999 999999999))
    (Class|PCGComponent|Cleanup (Variables|/Game/Village/BP_Village.BP_Village_C|GetPCG _returnvalue) false false)
    (PCG|Generate (Variables|/Game/Village/BP_Village.BP_Village_C|GetPCG _returnvalue) true)))

(event Input|KeyboardEvents|2
  (params (Key :type Key%20Structure :default "None"))
  (:Pressed
    (bind _returnvalue (Actor|GetActorOfClass "/Game/Village/BP_Forest.BP_Forest_C"))
    (Class|PCGGraphParametersHelpers|SetInt32Parameter (Variables|/Script/PCG.PCGComponent|GetGraphInstance (Variables|/Game/Village/BP_Forest.BP_Forest_C|GetPCG _returnvalue)) "ForestSEED" (Math|Random|RandomIntegerinRange -999999999 999999999))
    (Class|PCGComponent|Cleanup (Variables|/Game/Village/BP_Forest.BP_Forest_C|GetPCG _returnvalue) false false)
    (PCG|Generate (Variables|/Game/Village/BP_Forest.BP_Forest_C|GetPCG _returnvalue) true)))

(fn ConstructionScript)